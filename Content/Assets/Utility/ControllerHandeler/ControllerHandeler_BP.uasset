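; Handles controller connects and disconnects across menus, character select and gameplay, branching on InGameplay and InCharacterSelect flags.
; In menus it logs changes to an info widget and shows a warning when the active controller disconnects; character select also resets that player's panel on either change.
; In gameplay a disconnect pauses the game, toggles player input, removes pause menus and shows a per-player warning, resuming once all warnings clear.
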(event `self.ReceiveBeginPlay`
  (if (not (`self.In Gameplay`))
    (bind _returnvalue (`|CreateWidget` "/Game/Assets/Utility/ControllerHandeler/ControllerChangeInfoWindow.ControllerChangeInfoWindow_C"))
    (bind _output_get (set `self.Controller Change Info Window` _returnvalue))
    (`UserWidget.AddToViewport` _output_get 0)))

(event `self.OnControllerConnectionChange`
  (params (connected :type Boolean) (UserID :type Integer) (ControllerID :type Integer))
  (if (`self.In Gameplay`)
    (`self.Handle Game Pulls` connected ControllerID)
    (else
      (`self.Handle Standard Pulls` connected ControllerID)
      (if (`self.In Character Select`)
        (`self.Handle Character Select Pulls` ControllerID)))))

(fn `Handle Character Select Pulls`
  (params (`Controller Index` :type Integer))
  (bind _character_select_gui (`self.Character Select GUI`))
  (for _array_element (`|MakeArray` (`/Game/Levels/Menus/GUI/CharacterSelect/CharacterSelect.CharacterSelectPanel0` _character_select_gui) (`/Game/Levels/Menus/GUI/CharacterSelect/CharacterSelect.CharacterSelectPanel1` _character_select_gui) (`/Game/Levels/Menus/GUI/CharacterSelect/CharacterSelect.CharacterSelectPanel2` _character_select_gui) (`/Game/Levels/Menus/GUI/CharacterSelect/CharacterSelect.CharacterSelectPanel3` _character_select_gui))
    (if (== `Controller Index` (`/Game/Levels/Menus/GUI/CharacterSelect/CharacterSelectPanel.Owner Player Index` _array_element))
      (`/Game/Levels/Menus/GUI/CharacterSelect/CharacterSelectPanel.Reset Panel` _array_element)))
  (return))

(fn `Handle Game Pulls`
  (params (`Controller Connected` :type Boolean) (`Controller Index` :type Integer))
  (if `Controller Connected`
    ;[1 1 1] Loop thru windows to get window corresponding to connected player controller, remove window if match
    (bind _foundwidgets (`WidgetBlueprintLibrary.GetAllWidgetsOfClass` "/Game/Assets/Utility/ControllerHandeler/ActiveControllerChangeWindow.ActiveControllerChangeWindow_C" false))
    (for _array_element _foundwidgets
      (bind _returnvalue (`GameplayStatics.GetPlayerControllerID` (`UserWidget.GetOwningPlayer` _array_element)))
      (if (== _returnvalue `Controller Index`)
        (`Widget.RemoveFromParent` _array_element)))
    ;[1 1 1] if all windows are gone, re-enable input and  resume gameplay
    (bind _foundwidgets_2 (`WidgetBlueprintLibrary.GetAllWidgetsOfClass` "/Game/Assets/Utility/ControllerHandeler/ActiveControllerChangeWindow.ActiveControllerChangeWindow_C"))
    (if (== 0 (`KismetArrayLibrary.Array_Length` _foundwidgets_2))
      (bind _asastro_game_instance (cast `/Game/Assets/Utility/AstroGameInstance` (`GameplayStatics.GetGameInstance`)))
      (`/Game/Assets/Utility/AstroGameInstance.Toggle All Player Input` _asastro_game_instance false)
      (`GameplayStatics.SetGamePaused` false))
    (else
      ;[1 1 1] Pause game, create warning window and give control to player that dissconnected
      (`GameplayStatics.SetGamePaused` true)
      (bind _returnvalue_2 (`|CreateWidget` "/Game/Assets/Utility/ControllerHandeler/ActiveControllerChangeWindow.ActiveControllerChangeWindow_C" (`GameplayStatics.GetPlayerController` `Controller Index`)))
      (`TextBlock.SetText` (`/Game/Assets/Utility/ControllerHandeler/ActiveControllerChangeWindow.TextBlock_67` _returnvalue_2) (`KismetTextLibrary.Conv_StringToText` (`KismetStringLibrary.Concat_StrStr` "Player " (`KismetStringLibrary.Conv_IntToString` (+ `Controller Index` 1)) " Dissconnected, please plug it back in.")))
      (`UserWidget.AddToViewport` _returnvalue_2 100)
      (bind _asastro_game_instance_2 (cast `/Game/Assets/Utility/AstroGameInstance` (`GameplayStatics.GetGameInstance`)))
      (`/Game/Assets/Utility/AstroGameInstance.Toggle All Player Input` _asastro_game_instance_2 true)
      (bind _foundwidgets_3 (`WidgetBlueprintLibrary.GetAllWidgetsOfClass` "/Game/Levels/GameModes/GUI/PauseMenu.PauseMenu_C"))
      (for _array_element_2 _foundwidgets_3
        (`Widget.RemoveFromParent` _array_element_2))
      (return))))

(fn `Handle Standard Pulls`
  (params (`Controller Connected` :type Boolean) (`Controller Index` :type Integer))
  (bind _controller_change_info_window (`self.Controller Change Info Window`))
  (if `Controller Connected`
    ;[1 1 1] Controller Plugged In
    (`/Game/Assets/Utility/ControllerHandeler/ControllerChangeInfoWindow.Add Text` _controller_change_info_window (`KismetStringLibrary.Concat_StrStr` "Controller: " (`KismetStringLibrary.Conv_IntToString` (+ `Controller Index` 1)) " Connected"))
    ;[1 1 1] Check if error message was up already and if the controller that was plugged in was the active destroy the error window
    (bind _foundwidgets (`WidgetBlueprintLibrary.GetAllWidgetsOfClass` "/Game/Assets/Utility/ControllerHandeler/ActiveControllerChangeWindow.ActiveControllerChangeWindow_C"))
    (bind _output (`|GetArrayItem` _foundwidgets))
    (`/Engine/EditorBlueprintResources/StandardMacros.IsValid` _output
      (:`Is Valid`
        (bind _asastro_game_instance (cast `/Game/Assets/Utility/AstroGameInstance` (`GameplayStatics.GetGameInstance`)))
        (bind _is_active_controller (`/Game/Assets/Utility/AstroGameInstance.Is Active Controller` _asastro_game_instance `Controller Index`))
        (if _is_active_controller
          (`Widget.RemoveFromParent` _output)))
      (:`Is Not Valid`
        (return)))
    (else
      ;[1 1 1] Controller Dissconnected
      (`/Game/Assets/Utility/ControllerHandeler/ControllerChangeInfoWindow.Add Text` _controller_change_info_window (`KismetStringLibrary.Concat_StrStr` "Controller: " (`KismetStringLibrary.Conv_IntToString` (+ `Controller Index` 1)) " Disconnected"))
      ;[1 1 1] Check if dissconnected controller was active controller if so spawn warning message
      (bind _asastro_game_instance_2 (cast `/Game/Assets/Utility/AstroGameInstance` (`GameplayStatics.GetGameInstance`)))
      (bind _is_active_controller_2 (`/Game/Assets/Utility/AstroGameInstance.Is Active Controller` _asastro_game_instance_2 `Controller Index`))
      (if _is_active_controller_2
        (bind _returnvalue (`|CreateWidget` "/Game/Assets/Utility/ControllerHandeler/ActiveControllerChangeWindow.ActiveControllerChangeWindow_C"))
        (set `/Game/Assets/Utility/ControllerHandeler/ActiveControllerChangeWindow.Controller Change Info Window` (`self.Controller Change Info Window`) _returnvalue)
        (`UserWidget.AddToViewport` _returnvalue 0)
        (return)))))

(fn `UserConstructionScript`)